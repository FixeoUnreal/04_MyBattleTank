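; MyTank_BP is a player tank Blueprint that handles camera aiming and firing input.
; On BeginPlay it passes its Barrel and Turret components to setter functions defined outside the file.
; Azimuth input yaws a gimbal and elevation input pitches the spring arm, keeping the two rotation axes on separate components.
; Releasing the Fire action calls Fire, whose logic also lives outside this Blueprint.
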(event `self.ReceiveBeginPlay`
  (`self.SetBarrelReference` (`self.Barrel`))
  (`self.SetTurretReference` (`self.Turret`)))

(event `InputAxis|AimAzimuth`
  (params (AxisValue :type "Float (single-precision)"))
  ;[1 1 1] Input Binding
  (`SceneComponent.K2_AddLocalRotation` (`self.Azimuth Gimbal`) (`KismetMathLibrary.MakeRotator` 0.0 0.0 AxisValue) false false))

(event `InputAxis|AimElevation`
  (params (AxisValue :type "Float (single-precision)"))
  ;[1 1 1] Input Binding
  (`SceneComponent.K2_AddLocalRotation` (`self.SpringArm`) (`KismetMathLibrary.MakeRotator` 0.0 AxisValue) false false))

(event `InputAction|Fire`
  (params (Key :type "Key Structure"))
  ;[1 1 1] Input Binding
  (:`Released`
    (`self.Fire`)))

(fn `UserConstructionScript`)